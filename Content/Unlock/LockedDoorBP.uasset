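; A locked door Blueprint that swings open when unlocked.
; DoUnlock runs the parent logic, then plays the DoorSweep timeline.
; Each timeline update sets the Door's relative yaw to the sweep value scaled by MaxOpen.
; The finished handler only calls an empty DoNothing function and a timeline SetNewTime node.
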(event `self.ReceiveBeginPlay`
  (`parent.ReceiveBeginPlay`))

(event `self.DoUnlock`
  (`parent.DoUnlock`)
  (bind (_direction _sweepvar) (`Timeline|DoorSweep` :!label _label)
    (:`Update`
      (`SceneComponent.K2_SetRelativeRotation` (`self.Door`) (`KismetMathLibrary.MakeRotator` 0.0 0.0 (* _sweepvar (`self.MaxOpen`))) false false))
    (:`Finished`
      (`self.DoNothing`)
      (goto _label :!via `SetNewTime`))))

(fn `DoNothing`)

(fn `UserConstructionScript`
  (`parent.UserConstructionScript`))