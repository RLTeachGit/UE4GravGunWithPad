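; LockableBP is a lock that opens when the objects in its UnlockArray trigger UnlockEvent in array order.
; A correct trigger advances the index and plays a door unlock sound, while a wrong one resets the sequence.
; Each attempt sends success and step-progress feedback back through the current expected unlock object.
; BeginPlay reports empty or invalid entries, and DoUnlock itself only resets the lock on completion.
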(event `self.ReceiveBeginPlay`
  (bind _unlockarray (`self.UnlockArray`))
  (if (> (`KismetArrayLibrary.Array_Length` _unlockarray) 0)
    (for (_array_element _array_index) _unlockarray
      (`/Engine/EditorBlueprintResources/StandardMacros.IsValid` _array_element
        (:`Is Not Valid`
          (`KismetSystemLibrary.PrintString` (`KismetTextLibrary.Conv_TextToString` (`|FormatText` "{Name} Invalid Unlock[{Index}]" (`KismetTextLibrary.Conv_StringToText` (`KismetSystemLibrary.GetDisplayName` self)) (`KismetTextLibrary.Conv_IntToText` _array_index)))))))
    (else
      (`KismetSystemLibrary.PrintString` "Unlock Array Empty"))))

(event `DoNotifyUnlock`
  (params (isSucccess :type Boolean :default true))
  (bind _currentindex (`self.CurrentIndex`))
  (bind _unlockarray (`self.UnlockArray`))
  (`/Game/Unlock/UnlockBP.DoPlayerFeedback` (`|GetArrayItem` _unlockarray _currentindex) isSucccess (+ _currentindex 1) (`KismetArrayLibrary.Array_Length` _unlockarray) self))

(event `UnlockEvent`
  (params (UnlockBP :type "/Game/Unlock/UnlockBP Object Reference"))
  (bind _currentindex (`self.CurrentIndex`))
  (if (== UnlockBP (`|GetArrayItem` (`self.UnlockArray`) _currentindex))
    (`self.DoNotifyUnlock` true)
    (bind _result (`/Engine/EditorBlueprintResources/StandardMacros.IncrementInt` _currentindex)
      (:`  `
        (if (>= _result (`KismetArrayLibrary.Array_Length` (`self.UnlockArray`)))
          (`self.DoUnlock`))
        (`GameplayStatics.PlaySoundAtLocation` "/Game/Unlock/DoorUnlock.DoorUnlock" (`self.K2_GetActorLocation`) (struct) 1.0 1.0 0.0 null null null)))
    (else
      (`self.DoNotifyUnlock` false)
      (`self.ResetLock`))))

(event `ResetLock`
  (set `self.CurrentIndex` 0)
  (`KismetSystemLibrary.PrintString` "LockReset"))

(event `DoUnlock`
  (`self.ResetLock`))

(fn `UserConstructionScript`)