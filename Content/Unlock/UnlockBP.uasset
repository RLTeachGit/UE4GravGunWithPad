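; UnlockBP is an unlocker that notifies a linked Lockable when it is triggered.
; The Triggered event prints the name of the actor that hit it, then calls UnlockEvent on the Lockable, passing itself as the source.
; BeginPlay prints a warning naming the instance if no valid Lockable is linked, though Triggered makes the call without rechecking.
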(event `self.ReceiveBeginPlay`
  (`/Engine/EditorBlueprintResources/StandardMacros.IsValid` (`self.Lockable`)
    (:`Is Not Valid`
      (`KismetSystemLibrary.PrintString` (`KismetTextLibrary.Conv_TextToString` (`|FormatText` "{Name} Not linked to Unlockable" (`KismetTextLibrary.Conv_StringToText` (`KismetSystemLibrary.GetDisplayName` self))))))))

(event `Triggered`
  (params (Actor :type "Actor Object Reference"))
  (`KismetSystemLibrary.PrintString` (`KismetTextLibrary.Conv_TextToString` (`|FormatText` "Hit by {Actor}" (`KismetTextLibrary.Conv_StringToText` (`KismetSystemLibrary.GetDisplayName` Actor)))))
  (`/Game/Unlock/LockableBP.UnlockEvent` (`self.Lockable`) self))

(fn `UserConstructionScript`)