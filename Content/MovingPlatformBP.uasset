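; Moving platform Blueprint that carries its static mesh back and forth between its starting location and a target actor.
; BeginPlay caches the mesh's world location as the start point.
; Each Tick lerps to the EndPosition actor's current location, using a degree-based sine of game time scaled by Speed and remapped to 0–1.
; The move is unswept, and motion follows global time, so it begins partway along the path.
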(event `self.ReceiveBeginPlay`
  (set `self.StartPosition` (`SceneComponent.K2_GetComponentLocation` (`self.StaticMeshComponent`))))

(event `self.ReceiveTick`
  (params (DeltaSeconds :type "Float (single-precision)"))
  (`SceneComponent.K2_SetWorldLocation` (`self.StaticMeshComponent`) (`KismetMathLibrary.VLerp` (`self.StartPosition`) (`self.K2_GetActorLocation` (`self.EndPosition`)) (/ (+ (`KismetMathLibrary.DegSin` (* (`GameplayStatics.GetTimeSeconds`) (`self.Speed`))) 1.0) 2.0)) false false))

(fn `UserConstructionScript`)