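; Invisible collider actor that gives visual and audio feedback when the first-person character or a projectile hits it.
; BeginPlay turns the mesh's default material into a dynamic instance and stores it.
; A valid hit swaps in the hit material, plays audio and starts a short timer that restores the default.
; Comparing the current material against the default blocks retriggering while the hit material is showing.
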(event `self.ReceiveBeginPlay`
  ;[1 1 1] Make Default material into Instance so we can mess with it
  (bind _returnvalue (`PrimitiveComponent.CreateDynamicMaterialInstance` (`self.StaticMesh`) 0 null "None"))
  (bind _output_get (set `self.DefaultMaterial` _returnvalue))
  (`PrimitiveComponent.SetMaterial` (`self.StaticMesh`) 0 _output_get))

(event `self.ReceiveHit`
  (params (MyComp :type "PrimitiveComponent Object Reference") (Other :type "Actor Object Reference") (OtherComp :type "PrimitiveComponent Object Reference") (bSelfMoved :type Boolean) (HitLocation :type "Vector Structure") (HitNormal :type "Vector Structure") (NormalImpulse :type "Vector Structure") (Hit :type "HitResult Structure (by ref)"))
  ;[1 1 1] Either Player or Bullet has hit this
  (cast `/Game/FirstPersonBP/Blueprints/FirstPersonCharacter` Other
    (:`then`
      _)
    (:`CastFailed`
      (cast `/Game/FirstPersonBP/Blueprints/FirstPersonProjectile` Other)))
  ;;[1 1 1] Set Hit material
  (if (== (`self.DefaultMaterial`) (`PrimitiveComponent.GetMaterial` (`self.StaticMesh`) 0))
    (`PrimitiveComponent.SetMaterial` (`self.StaticMesh`) 0 (`self.HitMaterial`))
    ;;[1 1 1] Will call event after timout expires
    (`KismetSystemLibrary.K2_SetTimerDelegate` (delegate `Reset Material`) 1.0)
    (`AudioComponent.Play` (`self.Audio`) 0.0)))

(event `Reset Material`
  ;[1 1 1] Set old material back
  (`PrimitiveComponent.SetMaterial` (`self.StaticMesh`) 0 (`self.DefaultMaterial`)))

(fn `UserConstructionScript`)